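; Server-side game mode for a timed multiplayer Pacman arena, managing joins, logouts, kicks, spawning and round restarts.
; PostLogin registers each controller and sets up its lobby menu from GameInfoInstance settings, while spawns use random PlayerStarts.
; Tick counts down the round and, at zero, resets the timer and respawns everyone as Pacman.
; A Delay in Tick throttles EveryoneUpdate, which pushes player counts, time and the gathered player list to every ArenaPC.
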(event Custom|SpawnCharacter
  (params (PlayerController :type Player%20Controller%20Object%20Reference) (CharacterClass :type Character%20Class%20Reference) (ChangeStatus :type Boolean))
  (bind _returnvalue (Pawn|GetControlledPawn PlayerController))
  (bind _spawnpoints (Variables|ServerSettings|GetSpawnPoints))
  ;[1 1 1] Spawn character
  (if (not ChangeStatus)
    (Utilities|IsValid _returnvalue
      (:Is%20Valid
        (Actor|DestroyActor _returnvalue))
      (:Is%20Not%20Valid
        _))
    (bind _returnvalue_2 (Game|SpawnActorfromClass CharacterClass (Transformation|GetActorTransform (Utilities|Array|Get(acopy) _spawnpoints (Math|Random|RandomIntegerinRange 0 (- (Utilities|Array|Length _spawnpoints) 1)))) "Undefined" 0 0))
    (Pawn|Possess PlayerController _returnvalue_2)))

(event Custom|RunTimer
  ;[1 1 1] Timer
  (Networking|SwitchHasAuthority
    (:Authority
      (Variables|ServerSettings|SetTimeLeft (Variables|ServerSettings|GetGameTime))
      (Variables|ServerSettings|SetIsTimerActive? true))))

(event Custom|YouHaveBeenKicked
  (params (PlayerID :type Integer))
  ;[1 1 1] On Kicked
  (Default|Kicked (.AsArena%20PC (Utilities|Casting|CastToArenaPC (Utilities|Array|Get(acopy) (Variables|ServerSettings|GetAllPlayerControllers) PlayerID)))))

(event Custom|ReStart
  ;[1 1 1] THE GAME IS OVER
  (Variables|ServerSettings|SetIsTimerActive? true)
  (Variables|ServerSettings|SetTimeLeft (Variables|ServerSettings|GetGameTime))
  (bind _array_element (Utilities|Array|ForEachLoopwithBreak (Variables|ServerSettings|GetAllPlayerControllers))
    (:LoopBody
      (CallFunction|RespawnPlayer _array_element))
    (:Completed
      (CallFunction|EveryoneUpdate))))

(event Custom|EveryoneUpdate
  (bind _allplayercontrollers (Variables|ServerSettings|GetAllPlayerControllers))
  ;[1 1 1] Update Everyone
  (bind _output_get (Variables|ServerSettings|SetCurrentPlayers (Utilities|Array|Length (Variables|ServerSettings|GetAllPlayerControllers))))
  (if (> _output_get 0)
    (Utilities|Array|Clear (Variables|ServerSettings|GetConnectedPlayers))
    (for _array_element _allplayercontrollers
      (bind _asarena_pc (Utilities|Casting|CastToArenaPC _array_element))
      (bind _info (Default|GetSettings _asarena_pc))
      (Utilities|Array|Add (Variables|ServerSettings|GetConnectedPlayers) _info)
      (Default|UpdateNumberOfPlayers _asarena_pc (Variables|ServerSettings|GetCurrentPlayers) (Variables|ServerSettings|GetMaxPlayers))
      (Default|UpdateTimer _asarena_pc (Variables|ServerSettings|GetTimeLeft)))
    (for _array_element_2 _allplayercontrollers
      (bind _asarena_pc_2 (Utilities|Casting|CastToArenaPC _array_element_2))
      (Default|AddPlayerInfo _asarena_pc_2 (Variables|ServerSettings|GetConnectedPlayers)))))

(event Custom|GameOver
  ;[1 1 1] THE GAME IS OVER
  (CallFunction|ReStart))

(event Custom|RespawnPlayer
  (params (PlayerController :type Player%20Controller%20Object%20Reference))
  (bind _returnvalue (Pawn|GetControlledPawn PlayerController))
  (bind _spawnpoints (Variables|ServerSettings|GetSpawnPoints))
  ;[1 1 1] ReSpawn the player
  (Utilities|IsValid _returnvalue
    (:Is%20Valid
      (Actor|DestroyActor _returnvalue))
    (:Is%20Not%20Valid
      _))
  (bind _returnvalue_2 (Game|SpawnActorfromClass "/Game/Blueprints/Characters/Pacman.Pacman_C" (Transformation|GetActorTransform (Utilities|Array|Get(acopy) _spawnpoints (Math|Random|RandomIntegerinRange 0 (- (Utilities|Array|Length _spawnpoints) 1)))) "Undefined" 0 0))
  (Pawn|Possess PlayerController _returnvalue_2)
  (bind _asarena_pc (Utilities|Casting|CastToArenaPC PlayerController))
  (Default|UpdateCharacter _asarena_pc))

(event EventPostLogin
  (params (NewPlayer :type Player%20Controller%20Object%20Reference))
  ;[1 1 1] OnPosLogin - Setup Player Controller and Spawn Player
  (Networking|SwitchHasAuthority
    (:Authority
      (Utilities|Array|Add (Variables|ServerSettings|GetAllPlayerControllers) NewPlayer)
      (bind _outactors (Actor|GetAllActorsOfClass "/Script/Engine.PlayerStart"))
      (Variables|ServerSettings|SetSpawnPoints _outactors)
      (bind _asgame_info_instance (Utilities|Casting|CastToGameInfoInstance (Game|GetGameInstance)))
      (Variables|ServerSettings|SetServerName (Variables|/Game/Blueprints/AllLevels/GameInfoInstance.GameInfoInstance_C|GetServeName _asgame_info_instance))
      (Variables|ServerSettings|SetMaxPlayers (Variables|/Game/Blueprints/AllLevels/GameInfoInstance.GameInfoInstance_C|GetMax%20Players _asgame_info_instance))
      (bind _asarena_pc (Utilities|Casting|CastToArenaPC NewPlayer))
      (Default|InitialSetup _asarena_pc)
      (Default|SetupLobbyMenu _asarena_pc (Variables|ServerSettings|GetServerName))
      (CallFunction|EveryoneUpdate)
      (Utilities|FlowControl|Delay 0.2)
      (Default|UpdateTimer _asarena_pc (Variables|ServerSettings|GetTimeLeft)))))

(event EventBeginPlay
  ;[1 1 1] Begin Play
  (Networking|SwitchHasAuthority
    (:Authority
      (CallFunction|RunTimer))))

(event EventOnLogout
  (params (ExitingController :type Controller%20Object%20Reference))
  (bind _allplayercontrollers (Variables|ServerSettings|GetAllPlayerControllers))
  ;[1 1 1] Event OnLogout
  (bind (_array_element _array_index) (Utilities|Array|ForEachLoopwithBreak _allplayercontrollers :!label _label)
    (:LoopBody
      (if (== _array_element ExitingController)
        (goto _label Break)))
    (:Completed
      (Utilities|Casting|CastToArenaPC (Utilities|Array|Get(acopy) _allplayercontrollers _array_index))
      (Utilities|Array|RemoveIndex (Variables|ServerSettings|GetAllPlayerControllers) _array_index)
      (Utilities|Array|RemoveIndex (Variables|ServerSettings|GetConnectedPlayers) _array_index)
      (CallFunction|EveryoneUpdate))))

(event EventTick
  (params (DeltaSeconds :type Float%20%28single-precision%29))
  (Utilities|FlowControl|Sequence
    (:then_0
      ;[1 1 1] Timer
      (Networking|SwitchHasAuthority
        (:Authority
          (if (Variables|ServerSettings|GetIsTimerActive?)
            (bind _output_get (Variables|ServerSettings|SetTimeLeft (- (Variables|ServerSettings|GetTimeLeft) DeltaSeconds)))
            (if (not (> _output_get 0.0))
              (Variables|ServerSettings|SetIsTimerActive? false)
              (CallFunction|GameOver)
              (Development|PrintString "THE GAME IS OVER" true true "(R=0.000000,G=0.660000,B=1.000000,A=1.000000)" 1e+01))))))
    (:then_1
      ;[1 1 1] Update Score List
      (Utilities|FlowControl|Delay 1.0)
      (CallFunction|EveryoneUpdate))))

(fn ConstructionScript)