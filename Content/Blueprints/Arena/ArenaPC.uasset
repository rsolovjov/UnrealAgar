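; ArenaPC is the multiplayer arena's player controller, handling each player's lobby and Pacman character.
; It loads player settings from GameInfoInstance, has ArenaGM spawn the character, then applies avatar and nickname.
; It fills the lobby widget's player list, count and timer, relays chat through every controller, and swaps in a loading screen.
; Leaving or being kicked destroys the session; save-slot code is disconnected.
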(event Custom|InitialSetup
  ;[1 1 1] Initial Setup
  (CallFunction|SaveGameCheck)
  (CallFunction|CallUpdate (Variables|PlayerInfo|GetPlayersSettings) false))

(event Custom|UpdateTimer
  (params (TimeLeft :type Float%20%28single-precision%29))
  (bind _lobbymenuwb (Variables|Widgets|GetLobbyMenuWB))
  ;[1 1 1] UpdateTimer
  (Utilities|IsValid _lobbymenuwb
    (:Is%20Valid
      (Variables|/Game/Agar/UI/Arena/LobbyMenu.LobbyMenu_C|SetTimeLeft _lobbymenuwb TimeLeft))))

(event Custom|UpdateCharacter
  (bind _playerssettings (Variables|PlayerInfo|GetPlayersSettings))
  (bind (_myplayername _myplayerimage) (Utilities|Struct|BreakPlayerInfo _playerssettings))
  ;[1 1 1] Update Character
  (bind _aspacman (Utilities|Casting|CastToPacman (Pawn|GetControlledPawn)))
  (Default|SetAvatar _aspacman _myplayerimage)
  (Default|SetNickname _aspacman _myplayername))

(event Custom|ShowLoadingScreem
  ;[1 1 1] Show Loading Screen
  (Widget|RemovefromParent (Variables|Widgets|GetLobbyMenuWB))
  (bind _returnvalue (UserInterface|CreateWidget "/Game/Agar/UI/AllLevels/LoadingScreen.LoadingScreen_C" self))
  (UserInterface|Viewport|AddtoViewport _returnvalue 0))

(event Custom|UpdateChat
  (params (Sender :type Text) (Text :type Text))
  ;[1 1 1] Updates the Chat Display
  (Default|UpdateChatWindow (Variables|/Game/Agar/UI/Arena/LobbyMenu.LobbyMenu_C|GetChatWindow (Variables|Widgets|GetLobbyMenuWB)) Sender Text))

(event Custom|UpdateNumberOfPlayers
  (params (CurrentPlayers :type Integer) (MaxPlayers :type Integer))
  (bind _lobbymenuwb (Variables|Widgets|GetLobbyMenuWB))
  ;[1 1 1] Update Number Of Players
  (Utilities|IsValid _lobbymenuwb
    (:Is%20Valid
      (Variables|/Game/Agar/UI/Arena/LobbyMenu.LobbyMenu_C|SetPlayersDisplay _lobbymenuwb (Utilities|Text|FormatText "{CurrentPlayers} of {MaxPlayers}" (Utilities|Text|ToText(Integer) CurrentPlayers) (Utilities|Text|ToText(Integer) MaxPlayers))))))

(event Custom|SetupLobbyMenu
  (params (ServerName :type Text))
  ;[1 1 1] Setup Lobby Menu
  (Variables|Default|SetbShowMouseCursor true)
  (bind _returnvalue (UserInterface|CreateWidget "/Game/Agar/UI/Arena/LobbyMenu.LobbyMenu_C" 0 ServerName))
  (bind _output_get (Variables|Widgets|SetLobbyMenuWB _returnvalue))
  (UserInterface|Viewport|AddtoViewport _output_get 0)
  (Input|SetInputModeGameandUI self _output_get "DoNotLock" true))

(event Custom|AddPlayerInfo
  (params (ConnectedPlayersInfo :type Array%20of%20Player%20Info%20Structures))
  (bind _lobbymenuwb (Variables|Widgets|GetLobbyMenuWB))
  ;[1 1 1] Upadate Player List Window
  (Variables|PlayerInfo|SetAllConnectedPlayers ConnectedPlayersInfo)
  (Utilities|IsValid _lobbymenuwb
    (:Is%20Valid
      (Default|ClearPlayerList _lobbymenuwb)
      (for _array_element (Variables|PlayerInfo|GetAllConnectedPlayers)
        (Default|UpdatePlayerWindow (Variables|Widgets|GetLobbyMenuWB) _array_element)))))

(event Custom|Kicked
  ;[1 1 1] Back To Main Menu
  (Game|OpenLevel(byName) "MainMenu")
  (|DestroySession self))

(event Custom|GetChatMessage
  (params (TextToSend :type Text))
  ;[1 1 1] Chat Message
  (Variables|PlayerInfo|SetSenderText TextToSend)
  (Variables|PlayerInfo|SetSenderName (.MyPlayerName (Utilities|Struct|BreakPlayerInfo (Variables|PlayerInfo|GetPlayersSettings))))
  (bind _asarena_gm (Utilities|Casting|CastToArenaGM (Game|GetGameMode)))
  (for _array_element (Variables|/Game/Blueprints/Arena/ArenaGM.ArenaGM_C|GetAllPlayerControllers _asarena_gm)
    (bind _asarena_pc (Utilities|Casting|CastToArenaPC _array_element))
    (CallFunction|UpdateChat _asarena_pc (Variables|PlayerInfo|GetSenderName) (Variables|PlayerInfo|GetSenderText))))

(event Custom|CallUpdate
  (params (PlayerInfo :type Player%20Info%20Structure) (ChangedStatus? :type Boolean))
  (bind _returnvalue (Game|GetGameMode))
  (bind _asarena_gm (Utilities|Casting|CastToArenaGM _returnvalue))
  ;[1 1 1] Update
  (Variables|PlayerInfo|SetPlayersSettings PlayerInfo)
  (Default|SpawnCharacter _asarena_gm self (Variables|Default|GetChar) ChangedStatus?)
  (CallFunction|UpdateCharacter)
  (Default|EveryoneUpdate _asarena_gm))

(event EventEndPlay
  (params (EndPlayReason :type EEndPlayReason%20Enum :default "Destroyed"))
  ;[1 1 1] Back To Main Menu
  (|DestroySession self))

(event Input|KeyboardEvents|T
  (params (Key :type Key%20Structure))
  (bind _lobbymenuwb (Variables|Widgets|GetLobbyMenuWB))
  (bind _playerlist (Variables|/Game/Agar/UI/Arena/LobbyMenu.LobbyMenu_C|GetPlayerList _lobbymenuwb))
  ;[1 1 1] Toogle Lobby Menu
  (:Pressed
    (Utilities|FlowControl|FlipFlop
      (:A
        (Widget|SetVisibility _playerlist "Hidden"))
      (:B
        (Widget|SetVisibility _playerlist "Visible")))))

(fn ConstructionScript)

(fn SaveGameCheck
  (bind _asgame_info_instance (Utilities|Casting|CastToGameInfoInstance (Game|GetGameInstance)))
  (Variables|PlayerInfo|SetPlayersSettings (Variables|/Game/Blueprints/AllLevels/GameInfoInstance.GameInfoInstance_C|GetPlayerInfo _asgame_info_instance)))

(fn LoadGame
  (bind _asgame_info_instance (Utilities|Casting|CastToGameInfoInstance (Game|GetGameInstance)))
  (Variables|PlayerInfo|SetPlayersSettings (Variables|/Game/Blueprints/AllLevels/GameInfoInstance.GameInfoInstance_C|GetPlayerInfo _asgame_info_instance)))

(fn SaveGame
  (bind _asgame_info_instance (Utilities|Casting|CastToGameInfoInstance (Game|GetGameInstance)))
  (Variables|/Game/Blueprints/AllLevels/GameInfoInstance.GameInfoInstance_C|SetPlayerInfo _asgame_info_instance (Variables|PlayerInfo|GetPlayersSettings)))

(fn GetSettings
  (bind _playerssettings (Variables|PlayerInfo|GetPlayersSettings))
  (bind (_myplayername _myplayerimage _myplayercharacter _myplayercharacterimage _myplayerstatus) (Utilities|Struct|BreakPlayerInfo _playerssettings))
  (Utilities|IsValid (Variables|Default|GetCharacterRef)
    (:Is%20Valid
      _)
    (:Is%20Not%20Valid
      (bind _aspacman (Utilities|Casting|CastToPacman (Pawn|GetControlledPawn))
        (:then
          (Variables|Default|SetCharacterRef _aspacman))
        (:CastFailed
          (return _playerssettings)))))
  (return (Utilities|Struct|MakePlayerInfo _myplayername _myplayerimage _myplayercharacter _myplayercharacterimage _myplayerstatus (Variables|/Game/Blueprints/Characters/Pacman.Pacman_C|GetWeight (Variables|Default|GetCharacterRef)))))